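; BP_SaveGameGameModeBase is a game mode that drives saving and loading of game state and spawns test actors.
; On BeginPlay it enables input from player 0 and calls LoadGameState on the CustomGameState, then calls SaveGameState on it at EndPlay.
; Pressing Space spawns a BP_Player at a random position within a large cube around the origin and prints a confirmation.
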(event EventBeginPlay
  (Utilities|FlowControl|Sequence
    (:then_0
      (Input|EnableInput (Game|GetPlayerController 0)))
    (:then_1
      (bind _ascustom_game_state (Utilities|Casting|CastToCustomGameState (Game|GetGameState)))
      (Class|CustomGameState|LoadGameState _ascustom_game_state))))

(event EventEndPlay
  (params (EndPlayReason :type EEndPlayReason%20Enum :default "Destroyed"))
  (bind _ascustom_game_state (Utilities|Casting|CastToCustomGameState (Game|GetGameState)))
  (Class|CustomGameState|SaveGameState _ascustom_game_state))

(event Input|KeyboardEvents|SpaceBar
  (params (Key :type Key%20Structure :default "None"))
  (:Pressed
    (Game|SpawnActorfromClass "/Game/BP_Player.BP_Player_C" (Math|Transform|MakeTransform (Math|Vector|MakeVector (- (* (Math|Random|RandomFloat) 2e+04) 1e+04) (- (* (Math|Random|RandomFloat) 2e+04) 1e+04) (- (* (Math|Random|RandomFloat) 2e+04) 1e+04)) "0, 0, 0" "1,1,1") "Undefined" 0 0)
    (Development|PrintString "ACTOR CREATED")))

(fn ConstructionScript)